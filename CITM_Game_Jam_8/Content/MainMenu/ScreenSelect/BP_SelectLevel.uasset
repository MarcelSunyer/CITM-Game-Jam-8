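; BP_SelectLevel is a main menu actor for the level select screen, shown according to the player menu pawn's NewGame flag.
; BeginPlay caches the BP_PlayerMenu pawn, and Tick polls its flag.
; While the flag is set, the widget's owning actor is unhidden and a DoOnce resets.
; When it clears, the DoOnce hides the actor once after a short delay.
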(event `self.ReceiveBeginPlay`
  (bind _asbp_player_menu (cast `/Game/MainMenu/MainMenuToto/BP_PlayerMenu` (`GameplayStatics.GetPlayerPawn` 0)))
  (set `self.As BP Player Menu` _asbp_player_menu))

(event `self.ReceiveTick`
  (params (DeltaSeconds :type "Float (single-precision)"))
  (if (`/Game/MainMenu/MainMenuToto/BP_PlayerMenu.NewGame` (`self.As BP Player Menu`))
    (`self.SetActorHiddenInGame` (`ActorComponent.GetOwner` (`self.Widget`)) false)
    (goto _label :!via `Reset`)
    (else
      (`/Engine/EditorBlueprintResources/StandardMacros.DoOnce` false :!label _label
        (:`Completed`
          (`KismetSystemLibrary.Delay` 0.6)
          (`self.SetActorHiddenInGame` true))))))

(fn `UserConstructionScript`)